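; Helper actor that links left and right hand follower actors to the VR pawn's motion controllers, named as hand triggers.
; While VRPawn is unset, Tick waits briefly, finds the pawn with GetActorOfClass and calls AssignHandsFc.
; That function uses Set Follower Target to write each controller into the matching follower's Follow_Motion_Ctrl_Cmp_Bp component as its tracking target.
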(event EventBeginPlay)

(event Collision|EventActorBeginOverlap
  (params (OtherActor :type Actor%20Object%20Reference)))

(event EventTick
  (params (DeltaSeconds :type Float%20%28single-precision%29))
  (if (== (Variables|Default|GetVR%20Pawn) 0)
    (Utilities|FlowControl|Delay 0.2)
    (bind _returnvalue (Actor|GetActorOfClass "/Game/VRTemplate/Blueprints/VRPawn.VRPawn_C"))
    (Variables|Default|SetVR%20Pawn _returnvalue)
    (CallFunction|AssignHandsFc (Variables|Default|GetVR%20Pawn))))

(fn ConstructionScript)

(fn AssignHandsFc
  (params (VrPawnParam :type VR%20Pawn%20Object%20Reference))
  (Utilities|SetFollowerTarget (Variables|Default|GetLeft%20Hand%20Follower) (Variables|/Game/VRTemplate/Blueprints/VRPawn.VRPawn_C|GetMotionControllerLeft VrPawnParam)
    (:Out
      (Utilities|SetFollowerTarget (Variables|Default|GetRight%20Hand%20Follower) (Variables|/Game/VRTemplate/Blueprints/VRPawn.VRPawn_C|GetMotionControllerRight VrPawnParam)))))