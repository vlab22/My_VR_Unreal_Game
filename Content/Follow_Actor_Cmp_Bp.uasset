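; Actor component that makes its owning actor follow another actor's position.
; Each Tick, when FollowTarget is set, it snaps the owner to the target's location without sweep, offset or smoothing, leaving rotation untouched.
; It also prints the owner's display name and that location every frame as debug output.
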(event EventBeginPlay)

(event EventTick
  (params (DeltaSeconds :type Float%20%28single-precision%29))
  (bind _follow_target (Variables|Default|GetFollow%20Target))
  (bind _returnvalue (Transformation|GetActorLocation _follow_target))
  (if (!= (Variables|Default|GetFollow%20Target) 0)
    (Transformation|SetActorLocation (Components|GetOwner) _returnvalue false false)
    (Development|PrintString (Utilities|String|Append (Utilities|GetDisplayName (Components|GetOwner)) " pos: " (Utilities|String|ToString(Vector) _returnvalue)))))