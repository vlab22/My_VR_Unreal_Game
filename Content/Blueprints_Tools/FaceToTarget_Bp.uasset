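; Actor component that keeps its owning actor rotated to face a target actor.
; It caches the owner on BeginPlay, and a SetTarget event assigns the target.
; Every tick it snaps the owner's rotation to the look-at rotation toward the target's location, with no interpolation or validity check.
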(event EventBeginPlay
  (Variables|Default|SetOwner (Components|GetOwner)))

(event EventTick
  (params (DeltaSeconds :type Float%20%28single-precision%29))
  (Transformation|SetActorRotation (Variables|Default|GetOwner) (Math|Rotator|FindLookatRotation (Transformation|GetActorLocation (Variables|Default|GetOwner)) (Transformation|GetActorLocation (Variables|Default|GetTarget)))))

(event EventSetTarget
  (params (Target%20Param :type Actor%20Object%20Reference))
  (Variables|Default|SetTarget Target%20Param))