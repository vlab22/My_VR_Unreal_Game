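; Actor component tool that moves its owning actor toward a point in front of an assigned target actor.
; Each tick it projects that point along the target's forward vector by DistanceTowardsCamera.
; When the owner is farther from it than Gap, ActorMoveUpdate moves it there with sweep at Speed, then LastPos records the new location.
; SetTarget assigns the target.
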(event EventBeginPlay
  (Variables|Default|SetOwner (Components|GetOwner)))

(event EventTick
  (params (DeltaSeconds :type Float%20%28single-precision%29))
  (bind _distance_towards_camera (Variables|Default|GetDistance%20Towards%20Camera))
  (bind _target (Variables|Default|GetTarget))
  (bind _returnvalue (Transformation|GetActorRotation _target))
  (bind _returnvalue_2 (Transformation|GetActorLocation _target))
  (bind _returnvalue_3 (Math|Vector|GetForwardVector _returnvalue))
  (bind _returnvalue_4 (* _returnvalue_3 _distance_towards_camera))
  (bind _returnvalue_5 (+ _returnvalue_2 _returnvalue_4))
  (if (> (Math|Vector|Distance(Vector) (Transformation|GetActorLocation (Variables|Default|GetOwner)) _returnvalue_5) (Variables|Default|GetGap))
    (Class|ITween|ActorMoveUpdate (Variables|Default|GetOwner) _returnvalue_5 DeltaSeconds (Variables|Default|GetSpeed) false true "none" "noOrientationChange" 0 5.0 "none")
    (Variables|Default|SetLast%20Pos (Transformation|GetActorLocation (Variables|Default|GetOwner)))))

(event EventSetTarget
  (params (Target%20Param :type Actor%20Object%20Reference))
  (Variables|Default|SetTarget Target%20Param))